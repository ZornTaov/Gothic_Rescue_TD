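; Grenade projectile Blueprint that deals area damage to characters around its location, layered on a parent projectile class.
; DoDamage ignores its SingleTarget input, sphere-overlaps BaseCharacter pawns within ExplosionRadius, sends the full Damage to each IDamageable one through AffectHealth, and returns true.
; The event graph and construction script only call their parents, so this file does not show what triggers the explosion.
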(event EventBeginPlay
  (|CallParentFunction))

(event Collision|EventActorBeginOverlap
  (params (OtherActor :type Actor%20Object%20Reference))
  (|CallParentFunction OtherActor) ; This node is disabled and will not be called.\nDrag off pins to build functionality.
)

(event EventTick
  (params (DeltaSeconds :type Float%20%28single-precision%29))
  (|CallParentFunction DeltaSeconds) ; This node is disabled and will not be called.\nDrag off pins to build functionality.
)

(fn ConstructionScript
  (|CallParentFunction))

(fn DoDamage
  (params (SingleTarget :type Object%20Object%20Reference))
  (bind _outactors (Collision|SphereOverlapActors (Transformation|GetActorLocation) (Variables|Default|GetExplosionRadius) (Utilities|Array|MakeArray "ObjectTypeQuery3") "/Game/Character/BaseCharacter.BaseCharacter_C"))
  (for _array_element _outactors
    (if (Utilities|DoesObjectImplementInterface _array_element "/Game/Enemy/iDamageable.iDamageable_C")
      (Class|IDamageable|AffectHealth(Message) _array_element (Variables|Default|GetDamage))))
  (return true))