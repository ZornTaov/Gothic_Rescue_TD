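; Sliding door level part that opens when something enters its trigger box and closes when anything leaves.
; A locked door opens only for a HeroCharacter with a key card, consuming the card and unlocking the door.
; An Opened flag guards the skeletal mesh open and close animations.
; BeginPlay tints a dynamic material cyan if locked or white otherwise, and unlocking does not update the tint.
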(event OnComponentBeginOverlap(Box)
  (params (OverlappedComponent :type Primitive%20Component%20Object%20Reference) (OtherActor :type Actor%20Object%20Reference) (OtherComp :type Primitive%20Component%20Object%20Reference) (OtherBodyIndex :type Integer) (bFromSweep :type Boolean) (SweepResult :type Hit%20Result%20Structure%20%28by%20ref%29))
  (if (Variables|Door|GetLocked)
    (bind _ashero_character (Utilities|Casting|CastToHeroCharacter OtherActor))
    (if (Variables|/Game/Character/BaseCharacter.BaseCharacter_C|GetHasKeyCard _ashero_character)
      (Variables|/Game/Character/BaseCharacter.BaseCharacter_C|SetHasKeyCard _ashero_character false)
      (Variables|Door|SetLocked false)
      (if (not (Variables|Door|GetOpened)) :!label _label
        (Variables|Door|SetOpened true)
        (Components|Animation|PlayAnimation (Variables|SkeletalMeshActor|GetSkeletalMeshComponent) "/Game/LevelParts/SlidingDoor/SlideDoor_Anim_Open.SlideDoor_Anim_Open" false)))
    (else
      (goto _label))))

(event OnComponentEndOverlap(Box)
  (params (OverlappedComponent :type Primitive%20Component%20Object%20Reference) (OtherActor :type Actor%20Object%20Reference) (OtherComp :type Primitive%20Component%20Object%20Reference) (OtherBodyIndex :type Integer))
  (if (Variables|Door|GetOpened)
    (Variables|Door|SetOpened false)
    (Components|Animation|PlayAnimation (Variables|SkeletalMeshActor|GetSkeletalMeshComponent) "/Game/LevelParts/SlidingDoor/SlideDoor_Anim_Close.SlideDoor_Anim_Close" false)))

(event EventBeginPlay
  (bind _skeletalmeshcomponent (Variables|SkeletalMeshActor|GetSkeletalMeshComponent))
  (if (Variables|Door|GetLocked)
    (bind _returnvalue (Rendering|Material|CreateDynamicMaterialInstance _skeletalmeshcomponent 0 "/Game/LevelParts/SlidingDoor/Door.Door" "None" :!class /Script/Engine.PrimitiveComponent))
    (Rendering|Material|SetVectorParameterValue _returnvalue "BaseColor" "(R=0.000000,G=0.817432,B=1.000000,A=1.000000)" :!class /Script/Engine.MaterialInstanceDynamic)
    (else
      (bind _returnvalue_2 (Rendering|Material|CreateDynamicMaterialInstance _skeletalmeshcomponent 0 "/Game/LevelParts/SlidingDoor/Door.Door" "None" :!class /Script/Engine.PrimitiveComponent))
      (Rendering|Material|SetVectorParameterValue _returnvalue_2 "BaseColor" "(R=1.000000,G=1.000000,B=1.000000,A=1.000000)" :!class /Script/Engine.MaterialInstanceDynamic))))

(event Collision|EventActorBeginOverlap
  (params (OtherActor :type Actor%20Object%20Reference)))

(event EventTick
  (params (DeltaSeconds :type Float%20%28single-precision%29)))

(fn ConstructionScript)