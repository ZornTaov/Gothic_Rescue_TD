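; Smart nav link Blueprint that makes AI agents jump to the link's destination.
; When a BaseCharacter reaches the link, it is launched with a computed velocity that overrides its current horizontal and vertical motion.
; CalculateVelocity solves the ballistic arc for a set JumpDuration, using a hardcoded gravity value rather than the world's.
; A leftover debug string prints whenever any agent reaches the link.
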(event EventBeginPlay)

(event Collision|EventActorBeginOverlap
  (params (OtherActor :type Actor%20Object%20Reference)))

(event EventTick
  (params (DeltaSeconds :type Float%20%28single-precision%29)))

(event EventSmartLinkReached
  (params (Agent :type Actor%20Object%20Reference) (Destination :type Vector%20%28by%20ref%29 :default "0, 0, 0"))
  (Development|PrintString "Hello")
  (bind _asbase_character (Utilities|Casting|CastToBaseCharacter Agent))
  (bind _velocity (CallFunction|CalculateVelocity Destination (Transformation|GetActorLocation Agent) (Variables|Default|GetJump%20Duration)))
  (Character|LaunchCharacter _asbase_character _velocity true true))

(fn ConstructionScript)

(fn CalculateVelocity
  (params (Destination%20Location :type Vector) (Starting%20Location :type Vector) (Duration :type Float%20%28single-precision%29))
  (LocalVariables|SetinDuration Duration)
  (return (Math|Vector|MakeVector (/ (- (.x Destination%20Location) (.x Starting%20Location)) (LocalVariables|GetinDuration)) (/ (- (.y Destination%20Location) (.y Starting%20Location)) (LocalVariables|GetinDuration)) (/ (- (.z Destination%20Location) (+ (.z Starting%20Location) (* (Math|Float|Square (LocalVariables|GetinDuration)) -0.5 982.0))) (LocalVariables|GetinDuration)))))