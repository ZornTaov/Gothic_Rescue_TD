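; Forklift level part that slides its static mesh between a starting point and an ending point when triggered.
; MoveForward plays a timeline that lerps the mesh's relative location between the two point components, and MoveBackwards reverses that same timeline.
; The timeline's Finished output calls the ForkliftMoved dispatcher to signal that the move is complete.
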(event Custom|MoveBackwards
  (bind _newtrack_0 (Timeline|Timeline_0 Reverse)
    (:Update
      (Transformation|SetRelativeLocation (Variables|Default|GetStaticMesh) (Math|Vector|Lerp(Vector) (Variables|/Script/Engine.SceneComponent|GetRelativeLocation (Variables|Default|GetStartingPoint)) (Variables|/Script/Engine.SceneComponent|GetRelativeLocation (Variables|Default|GetEndingPoint)) _newtrack_0) false false))
    (:Finished
      (Default|CallForkliftMoved))))

(event Custom|MoveForward
  (bind _newtrack_0 (Timeline|Timeline_0 Play)
    (:Update
      (Transformation|SetRelativeLocation (Variables|Default|GetStaticMesh) (Math|Vector|Lerp(Vector) (Variables|/Script/Engine.SceneComponent|GetRelativeLocation (Variables|Default|GetStartingPoint)) (Variables|/Script/Engine.SceneComponent|GetRelativeLocation (Variables|Default|GetEndingPoint)) _newtrack_0) false false))
    (:Finished
      (Default|CallForkliftMoved))))

(event EventBeginPlay)

(event Collision|EventActorBeginOverlap
  (params (OtherActor :type Actor%20Object%20Reference)))

(event EventTick
  (params (DeltaSeconds :type Float%20%28single-precision%29)))

(fn ConstructionScript)