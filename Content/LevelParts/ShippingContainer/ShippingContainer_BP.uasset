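; Shipping container level prop with animated doors that open and close on the left, right or both sides.
; Six custom events each play a non-looping animation on the skeletal mesh, wait a fixed delay, then switch to an end-state animation.
; OpenBoth differs by replaying its opening animation after the delay.
; Door state is not tracked, and nothing in this Blueprint calls the events.
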(event Custom|CloseBoth
  (bind _skeletalmesh (Variables|Default|GetSkeletalMesh))
  (Components|Animation|PlayAnimation _skeletalmesh "/Game/LevelParts/ShippingContainer/shipping_container_Both_Closing.shipping_container_Both_Closing" false)
  (Utilities|FlowControl|Delay 1.3)
  (Components|Animation|PlayAnimation _skeletalmesh "/Game/LevelParts/ShippingContainer/shipping_container_Closed.shipping_container_Closed" false))

(event Custom|OpenRight
  (bind _skeletalmesh (Variables|Default|GetSkeletalMesh))
  (Components|Animation|PlayAnimation _skeletalmesh "/Game/LevelParts/ShippingContainer/shipping_container_Right.shipping_container_Right" false)
  (Utilities|FlowControl|Delay 1.3)
  (Components|Animation|PlayAnimation _skeletalmesh "/Game/LevelParts/ShippingContainer/shipping_container_RightOpen.shipping_container_RightOpen" false))

(event Custom|CloseRight
  (bind _skeletalmesh (Variables|Default|GetSkeletalMesh))
  (Components|Animation|PlayAnimation _skeletalmesh "/Game/LevelParts/ShippingContainer/shipping_container_Right_Closing.shipping_container_Right_Closing" false)
  (Utilities|FlowControl|Delay 1.3)
  (Components|Animation|PlayAnimation _skeletalmesh "/Game/LevelParts/ShippingContainer/shipping_container_Closed.shipping_container_Closed" false))

(event Custom|OpenLeft
  (bind _skeletalmesh (Variables|Default|GetSkeletalMesh))
  (Components|Animation|PlayAnimation _skeletalmesh "/Game/LevelParts/ShippingContainer/shipping_container_Left.shipping_container_Left" false)
  (Utilities|FlowControl|Delay 1.3)
  (Components|Animation|PlayAnimation _skeletalmesh "/Game/LevelParts/ShippingContainer/shipping_container_LeftOpen.shipping_container_LeftOpen" false))

(event Custom|CloseLeft
  (bind _skeletalmesh (Variables|Default|GetSkeletalMesh))
  (Components|Animation|PlayAnimation _skeletalmesh "/Game/LevelParts/ShippingContainer/shipping_container_Left_Closing.shipping_container_Left_Closing" false)
  (Utilities|FlowControl|Delay 1.3)
  (Components|Animation|PlayAnimation _skeletalmesh "/Game/LevelParts/ShippingContainer/shipping_container_Closed.shipping_container_Closed" false))

(event Custom|OpenBoth
  (bind _skeletalmesh (Variables|Default|GetSkeletalMesh))
  (Components|Animation|PlayAnimation _skeletalmesh "/Game/LevelParts/ShippingContainer/shipping_container_Both.shipping_container_Both" false)
  (Utilities|FlowControl|Delay 1.3)
  (Components|Animation|PlayAnimation _skeletalmesh "/Game/LevelParts/ShippingContainer/shipping_container_Both.shipping_container_Both" false))

(event EventBeginPlay)

(fn ConstructionScript)