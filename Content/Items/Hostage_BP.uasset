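; Hostage pickup actor that the hero collects by walking into its skeletal mesh.
; On the first overlap by a HeroCharacter without a hostage, it flags the hero, disables mesh physics simulation, and attaches itself to the hero's BackSocket with a dangling animation.
; It then reuses the WinScreen widget to briefly show a return-to-drop-point objective, hiding it after a delay.
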(event OnComponentBeginOverlap(SkeletalMesh)
  (params (OverlappedComponent :type Primitive%20Component%20Object%20Reference) (OtherActor :type Actor%20Object%20Reference) (OtherComp :type Primitive%20Component%20Object%20Reference) (OtherBodyIndex :type Integer) (bFromSweep :type Boolean) (SweepResult :type Hit%20Result%20Structure%20%28by%20ref%29))
  (bind _ashero_character (Utilities|Casting|CastToHeroCharacter OtherActor))
  (if (not (Variables|/Game/Character/HeroCharacter.HeroCharacter_C|GetHasHostage _ashero_character))
    (Utilities|FlowControl|DoOnce false
      (:Completed
        (Variables|/Game/Character/HeroCharacter.HeroCharacter_C|SetHasHostage _ashero_character true)
        (Physics|SetSimulatePhysics (Variables|Default|GetSkeletalMesh) false)
        (Collision|SetCollisionEnabled (Variables|Default|GetSkeletalMesh) "PhysicsOnly")
        (Transformation|AttachComponentToComponent (Variables|Default|GetSkeletalMesh) (Variables|/Script/Engine.Character|GetMesh _ashero_character) "BackSocket" "SnapToTarget" "SnapToTarget" "SnapToTarget" true)
        (Components|Animation|PlayAnimation (Variables|Default|GetSkeletalMesh) "/Game/Items/Hostage/dangling_Anim.dangling_Anim" false)
        (bind _returnvalue (UserInterface|CreateWidget "/Game/Character/WinScreen.WinScreen_C" (Game|GetPlayerController 0)))
        (Default|SetScreenText _returnvalue "Return the Hostage 
to the Drop Point.")
        (UserInterface|Viewport|AddtoViewport _returnvalue 0)
        (Utilities|FlowControl|Delay 3.0)
        (Widget|SetVisibility _returnvalue "Hidden")))))

(event EventBeginPlay)

(event EventTick
  (params (DeltaSeconds :type Float%20%28single-precision%29)))

(fn ConstructionScript)