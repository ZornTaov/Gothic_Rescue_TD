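; Base cover object that tells overlapping actors when cover is available and when they reach either end of it.
; The main cover box reports availability through CoverInterface, passing the cover arrow's world rotation on entry and clearing it on exit.
; Separate left and right boxes send end-of-cover flags for their side on overlap, and reset both flags when the actor leaves.
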(event OnComponentBeginOverlap(CoverBox)
  (params (OverlappedComponent :type Primitive%20Component%20Object%20Reference) (OtherActor :type Actor%20Object%20Reference) (OtherComp :type Primitive%20Component%20Object%20Reference) (OtherBodyIndex :type Integer) (bFromSweep :type Boolean) (SweepResult :type Hit%20Result%20Structure%20%28by%20ref%29))
  ;[1 1 1] CoverBox
  (if (Utilities|DoesObjectImplementInterface OtherActor (Variables|Default|GetCoverInterface))
    (Class|ICover|IsCoverAvailable(Message) OtherActor true (Transformation|GetWorldRotation (Variables|Default|GetCoverArrow)))))

(event OnComponentEndOverlap(CoverBox)
  (params (OverlappedComponent :type Primitive%20Component%20Object%20Reference) (OtherActor :type Actor%20Object%20Reference) (OtherComp :type Primitive%20Component%20Object%20Reference) (OtherBodyIndex :type Integer))
  ;[1 1 1] CoverBox
  (if (Utilities|DoesObjectImplementInterface OtherActor (Variables|Default|GetCoverInterface))
    (Class|ICover|IsCoverAvailable(Message) OtherActor false "0, 0, 0")))

(event OnComponentBeginOverlap(CoverBoxLeft)
  (params (OverlappedComponent :type Primitive%20Component%20Object%20Reference) (OtherActor :type Actor%20Object%20Reference) (OtherComp :type Primitive%20Component%20Object%20Reference) (OtherBodyIndex :type Integer) (bFromSweep :type Boolean) (SweepResult :type Hit%20Result%20Structure%20%28by%20ref%29))
  ;[1 1 1] CoverBoxLeft
  (if (Utilities|DoesObjectImplementInterface OtherActor (Variables|Default|GetCoverInterface))
    (Class|ICover|EndOfCover(Message) OtherActor true false)))

(event OnComponentEndOverlap(CoverBoxLeft)
  (params (OverlappedComponent :type Primitive%20Component%20Object%20Reference) (OtherActor :type Actor%20Object%20Reference) (OtherComp :type Primitive%20Component%20Object%20Reference) (OtherBodyIndex :type Integer))
  ;[1 1 1] CoverBoxLeft
  (if (Utilities|DoesObjectImplementInterface OtherActor (Variables|Default|GetCoverInterface))
    (Class|ICover|EndOfCover(Message) OtherActor false false)))

(event OnComponentBeginOverlap(CoverBoxRight)
  (params (OverlappedComponent :type Primitive%20Component%20Object%20Reference) (OtherActor :type Actor%20Object%20Reference) (OtherComp :type Primitive%20Component%20Object%20Reference) (OtherBodyIndex :type Integer) (bFromSweep :type Boolean) (SweepResult :type Hit%20Result%20Structure%20%28by%20ref%29))
  ;[1 1 1] CoverBoxRight
  (if (Utilities|DoesObjectImplementInterface OtherActor (Variables|Default|GetCoverInterface))
    (Class|ICover|EndOfCover(Message) OtherActor false true)))

(event OnComponentEndOverlap(CoverBoxRight)
  (params (OverlappedComponent :type Primitive%20Component%20Object%20Reference) (OtherActor :type Actor%20Object%20Reference) (OtherComp :type Primitive%20Component%20Object%20Reference) (OtherBodyIndex :type Integer))
  ;[1 1 1] CoverBoxRight
  (if (Utilities|DoesObjectImplementInterface OtherActor (Variables|Default|GetCoverInterface))
    (Class|ICover|EndOfCover(Message) OtherActor false false)))

(fn ConstructionScript)