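; Enemy Blueprint that has patrol waypoints and switches to Combat when PawnSensing sees or hears a TwinStickPawn, storing it as the player.
; FireWeapon branches on CombatType: Assault runs a looping-timer shotgun that spawns cone-spread projectiles and pauses after several bursts, while Cover's rifle event is empty.
; The construction script shows waypoint billboards for patrollers, sets the weapon mesh, and attaches it and the muzzle arrow to the weapon socket.
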(event OnSeePawn(PawnSensing)
  (params (Pawn :type Pawn%20Object%20Reference))
  (CallFunction|SettoCombat Pawn))

(event OnHearNoise(PawnSensing)
  (params (Instigator :type Pawn%20Object%20Reference) (Location :type Vector%20%28by%20ref%29 :default "0, 0, 0") (Volume :type Float%20%28single-precision%29))
  (CallFunction|SettoCombat Instigator))

(event Custom|FireWeapon
  (if (not (Variables|Default|GetisDead))
    (switch Utilities|FlowControl|Switch|SwitchonCombatType_Enum (Variables|Default|GetCombatType)
      (:NewEnumerator0
        (CallFunction|FireShotgun))
      (:NewEnumerator1
        (CallFunction|FireRifle)))))

(event Custom|StopFireWeapon
  (Utilities|Time|ClearandInvalidateTimerbyHandle (Variables|Weapon|GetTimerHandle)))

(event Custom|FireShotgun
  ;[1 1 1] Shotgun
  (CallFunction|ShotgunBurst)
  (bind _returnvalue (Utilities|Time|SetTimerbyEvent (delegate Custom|ShotgunBurst) 1.0 true))
  (Variables|Weapon|SetTimerHandle _returnvalue))

(event Custom|FireRifle)

(event Custom|ShotgunBurst
  ;[1 1 1] Shotgun
  (if (< (Variables|Weapon|GetFireCount) 3)
    (Components|Animation|PlayAnimation (Variables|Default|GetWeaponMesh) "/Game/AnimStarterPack/Fire_Shotgun_Hip.Fire_Shotgun_Hip" false)
    (for _index (range 1 (Variables|Shotgun|GetShotgunBurstCount))
      (bind _projectilespawninfo (CallFunction|CalculateShotgunFire))
      (bind _returnvalue (Game|SpawnActorfromClass "/Game/Weapons/Projectile/ShotgunProjectile.ShotgunProjectile_C" _projectilespawninfo "AlwaysSpawn" 0 self))
      (Variables|/Game/Weapons/Projectile/ShotgunProjectile.ShotgunProjectile_C|Setshooter _returnvalue self)
      (Audio|PlaySoundatLocation "/Game/TwinStick/Audio/TwinStickFire.TwinStickFire" (.Location (Math|Transform|BreakTransform _projectilespawninfo)) "0, 0, 0" 1.0 1.0 0.0 0 0 0))
    (Variables|Weapon|SetFireCount (+ (Variables|Weapon|GetFireCount) 1))
    (else
      (Utilities|FlowControl|Delay 3.0)
      (Variables|Weapon|SetFireCount 0))))

(event EventBeginPlay
  (Variables|Default|SetWaypoint1 (Transformation|GetWorldLocation (Variables|Default|GetWaypoint%202%20Billboard)))
  (Variables|Default|SetWaypoint2 (Transformation|GetWorldLocation (Variables|Default|GetWaypoint%201%20Billboard))))

(event Collision|EventActorBeginOverlap
  (params (OtherActor :type Actor%20Object%20Reference)))

(event EventTick
  (params (DeltaSeconds :type Float%20%28single-precision%29)))

(fn ConstructionScript
  (bind _weaponmesh (Variables|Default|GetWeaponMesh))
  (Utilities|FlowControl|Sequence
    (:then_0
      (switch Utilities|FlowControl|Switch|SwitchonCombatStatus_Enum (Variables|Default|GetCombatStatus)
        (:NewEnumerator1
          (Rendering|SetVisibility (Variables|Default|GetWaypoint%201%20Billboard) true false)
          (Rendering|SetVisibility (Variables|Default|GetWaypoint%202%20Billboard) true false))))
    (:then_1
      (switch Utilities|FlowControl|Switch|SwitchonCombatType_Enum (Variables|Default|GetCombatType)
        (:NewEnumerator0
          (Class|SkinnedMeshComponent|SetSkeletalMesh _weaponmesh "/Engine/EngineMeshes/SkeletalCube.SkeletalCube" true))
        (:NewEnumerator1
          (Class|SkinnedMeshComponent|SetSkeletalMesh _weaponmesh "/Engine/EngineMeshes/SkeletalCube.SkeletalCube" true))
        (:NewEnumerator2
          (Class|SkinnedMeshComponent|SetSkeletalMesh _weaponmesh "/Engine/EngineMeshes/SkeletalCube.SkeletalCube" true))))
    (:then_2
      (Transformation|AttachComponentToComponent (Variables|Default|GetWeaponMesh) (Variables|Character|GetMesh) "WeaponSocket" "SnapToTarget" "SnapToTarget" "KeepWorld" true))
    (:then_3
      (Transformation|AttachComponentToComponent (Variables|Default|GetMuzzleArrow) (Variables|Character|GetMesh) "WeaponSocket" "SnapToTarget" "SnapToTarget" "KeepWorld" true))))

(fn SettoCombat
  (params (SensedPawn :type Object%20Object%20Reference))
  (if (not (Utilities|Enum|Equal(Enum) (Variables|Default|GetCombatStatus) "NewEnumerator2"))
    (bind _astwin_stick_pawn (Utilities|Casting|CastToTwinStickPawn SensedPawn))
    (Variables|Default|SetPlayerCharacter _astwin_stick_pawn)
    (Variables|Default|SetCombatStatus "NewEnumerator2")))

(fn CalculateShotgunFire
  (bind _muzzlearrow (Variables|Default|GetMuzzleArrow))
  (bind _shotgunspread (Variables|Shotgun|GetShotgunSpread))
  (bind _returnvalue (Math|Vector|GetForwardVector _muzzlearrow))
  (bind _returnvalue_2 (Math|Random|RandomUnitVectorinConeinDegrees _returnvalue _shotgunspread))
  (bind _returnvalue_3 (Math|Conversions|RotationFromXVector _returnvalue_2))
  (return (Math|Transform|MakeTransform (+ (Math|Vector|RotateVector "85.000000, 0, 0" _returnvalue_3) (Transformation|GetWorldLocation _muzzlearrow)) _returnvalue_3 "1.000000,1.000000,1.000000")))